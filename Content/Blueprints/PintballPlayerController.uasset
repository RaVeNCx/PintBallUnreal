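; Player controller for a pinball game that drives the table's flippers from player input.
; On BeginPlay it finds every Flipper actor in the level and sorts it by FlipType into left and right arrays.
; The LeftFlipper action calls Flop on each left flipper when pressed and Flip when released.
; The right array is filled, but no input here uses it.
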(event Custom|DefectFlippers
  (bind _outactors (Actor|GetAllActorsOfClass "/Game/Blueprints/Flipper.Flipper_C"))
  (for _array_element _outactors
    (switch Utilities|FlowControl|Switch|SwitchonFlipType (Variables|/Game/Blueprints/Flipper.Flipper_C|GetFlipType _array_element)
      (:NewEnumerator0
        (Utilities|Array|Add (Variables|Default|GetLeftFlppers) _array_element))
      (:NewEnumerator1
        (Utilities|Array|Add (Variables|Default|GetRightFlppers) _array_element)))))

(event EventBeginPlay
  (CallFunction|DefectFlippers))

(event EventTick
  (params (DeltaSeconds :type Float%20%28single-precision%29)))

(event Input|ActionEvents|InputActionLeftFlipper
  (params (Key :type Key%20Structure :default "None"))
  (bind _leftflppers (Variables|Default|GetLeftFlppers))
  (:Pressed
    (for _array_element _leftflppers
      (Default|Flop _array_element)))
  (:Released
    (for _array_element_2 _leftflppers
      (Default|Flip _array_element_2))))

(fn ConstructionScript)